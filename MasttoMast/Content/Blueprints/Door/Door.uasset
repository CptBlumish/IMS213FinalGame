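; Door Blueprint that opens by sliding down once enough items have been collected.
; CollectItem increments a counter and, when it reaches MaxItemsCollected, triggers DoorDown through a DoOnce so it fires only one time.
; DoorDown plays the Down timeline, lerping the Cube's relative Z location to lower it out of the way.
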(event `DoorDown`
  (bind (_direction _slidedown) (`Timeline|Down`)
    (:`Update`
      (`SceneComponent.K2_SetRelativeLocation` (`self.Cube`) (`KismetMathLibrary.MakeVector` 0.0 0.0 (`KismetMathLibrary.Lerp` 0.0 -1450.0 _slidedown)) false false))))

(event `CollectItem`
  (`/Engine/EditorBlueprintResources/StandardMacros.IncrementInt` (`self.CurrentItemsCollected`)
    (:`  `
      (if (== (`self.CurrentItemsCollected`) (`self.MaxItemsCollected`))
        (`/Engine/EditorBlueprintResources/StandardMacros.DoOnce` false
          (:`Completed`
            (`self.DoorDown`)))))))

(fn `UserConstructionScript`)